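; USPawn is a pawn Blueprint that swaps its mesh between first-person and third-person versions.
; SetFirstPersonCamera runs only with authority, stores the IsFirstPerson flag and sets Mesh to Mesh1p or Mesh3p, printing a message if the chosen mesh is invalid.
; It changes no camera component despite the function's name, and its event graph and construction script are empty.
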(event EventBeginPlay)

(event Collision|EventActorBeginOverlap
  (params (OtherActor :type Actor%20Object%20Reference)))

(event EventTick
  (params (DeltaSeconds :type Float%20%28single-precision%29)))

(fn ConstructionScript)

(fn SetFirstPersonCamera
  (params (FirstPerson :type Boolean))
  (bind _mesh (Variables|Default|GetMesh))
  (bind _mesh1p (Variables|Default|GetMesh1p))
  (bind _mesh3p (Variables|Default|GetMesh3p))
  (Networking|SwitchHasAuthority
    (:Authority
      (bind _output_get (Variables|Default|SetIsFirstPerson FirstPerson))
      (if _output_get
        (Utilities|IsValid _mesh1p
          (:Is%20Valid
            (Components|StaticMesh|SetStaticMesh _mesh _mesh1p))
          (:Is%20Not%20Valid
            (Development|PrintText "Mesh1p is invalid")))
        (else
          (Utilities|IsValid _mesh3p
            (:Is%20Valid
              (Components|StaticMesh|SetStaticMesh _mesh _mesh3p))
            (:Is%20Not%20Valid
              (Development|PrintText "Mesh3p is invalid"))))))))